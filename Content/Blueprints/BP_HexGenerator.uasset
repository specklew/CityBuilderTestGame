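; BP_HexGenerator builds a hex tile map with a scaled water plane at construction, as instanced meshes or child tile actors.
; Rows alternate offsets to form the hex grid.
; FastNoise sets instance heights, separating flat land from varied water depths and storing height in custom data; it also prepares seeded decor noise per tile type.
; In instanced mode, clicking collapses the hit tile to zero scale; a debug function prints tile-type counts.
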(event EventBeginPlay
  (if (Variables|GridOptions|GetIsInstanced)
    (Input|EnableInput (Game|GetPlayerController 0))))

(event Input|MouseEvents|LeftMouseButton
  (params (Key :type Key%20Structure))
  (:Released
    (if (Variables|GridOptions|GetIsInstanced)
      (bind _output_get (Variables|Hidden|SetHit%20Item%20Index (.HitItem (Collision|BreakHitResult (.HitResult (Game|Player|GetHitResultUnderCursorbyChannel (Game|GetPlayerController 0) "TraceTypeQuery1" true))))))
      (Development|PrintString (Utilities|String|ToString(Integer) _output_get))
      (Components|InstancedStaticMesh|UpdateInstanceTransform (Variables|Default|GetInstancedStaticMesh) (Variables|Hidden|GetHit%20Item%20Index) (Math|Transform|MakeTransform (.Location (Math|Transform|BreakTransform (.OutInstanceTransform (Components|InstancedStaticMesh|GetInstanceTransform (Variables|Default|GetInstancedStaticMesh) _output_get false)))) (.Rotation (Math|Transform|BreakTransform (.OutInstanceTransform (Components|InstancedStaticMesh|GetInstanceTransform (Variables|Default|GetInstancedStaticMesh) _output_get false)))) "0.000000,0.000000,0.000000") true true false))))

(fn ConstructionScript
  (CallFunction|SetNoiseWrappers)
  (Variables|Hidden|SetRadius (* (.X (Math|Vector|BreakVector (.Max (Utilities|Struct|BreakBox (StaticMesh|GetBoundingBox (Variables|GridOptions|GetTile%20Mesh)))))) (Variables|GridOptions|GetScale)))
  ;[1 0 0.006409] Height Loop
  (for _index (range 0 (- (Variables|GridOptions|GetHeight) 1))
    ;[1 0.008232 0] Width Loop
    (for _index_2 (range 0 (- (Variables|GridOptions|GetWidth) 1))
      (if (Variables|GridOptions|GetIsInstanced)
        ;[1 0.7267 0] Instanced Static Mesh
        (bind _returnvalue (Components|InstancedStaticMesh|AddInstance (Variables|Default|GetInstancedStaticMesh) (Math|Transform|MakeTransform (Math|Vector|MakeVector (+ (* _index_2 (Variables|Hidden|GetRadius) 2.0) (* _index_2 (Variables|GridOptions|GetOffset)) (Variables|Hidden|GetRow%20Offset)) (+ (* _index (/ (* (Variables|Hidden|GetRadius) 2.0) (Math|Float|Sqrt 3.0)) 1.5) (* _index (Variables|GridOptions|GetOffset))) 0.0) "0, 0, 0" (Math|Conversions|ToVector(Float) (Variables|GridOptions|GetScale))) false))
        (Variables|Hidden|SetInstance%20Index _returnvalue)
        (CallFunction|UpdateInstancedStaticMesh)
        (else
          ;[1 0 0.7703] Child Actor Component
          (bind _returnvalue_2 (AddComponent|AddChildActorComponent false (Math|Transform|MakeTransform (Math|Vector|MakeVector (+ (* _index_2 (Variables|Hidden|GetRadius) 2.0) (* _index_2 (Variables|GridOptions|GetOffset)) (Variables|Hidden|GetRow%20Offset)) (+ (* _index (/ (* (Variables|Hidden|GetRadius) 2.0) (Math|Float|Sqrt 3.0)) 1.5) (* _index (Variables|GridOptions|GetOffset))) 0.0) "0, 0, 0" (Math|Conversions|ToVector(Float) (Variables|GridOptions|GetScale)))))
          (ChildActorComponent|SetChildActorClass _returnvalue_2 (Variables|NormalTileOptions|GetHex%20Tile%20Class)))))
    ;[0 1 0.008149] Offset Every Second Row
    (Utilities|FlowControl|FlipFlop
      (:A
        (Variables|Hidden|SetRow%20Offset (* (Variables|Hidden|GetRadius) -1.0)))
      (:B
        (Variables|Hidden|SetRow%20Offset 0.0))))
  ;[0 0.1222 1] Scale Water
  (Transformation|SetWorldTransform (Variables|Default|GetStaticMesh) (Math|Transform|MakeTransform (- (Transformation|GetActorLocation self) (Math|Vector|MakeVector (Variables|Hidden|GetRadius) (Variables|Hidden|GetRadius) 0.0)) "0, 0, 0" (* (/ (Variables|Hidden|GetRadius) (.X (Math|Vector|BreakVector (.Max (Utilities|Struct|BreakBox (StaticMesh|GetBoundingBox (Variables|/Script/Engine.StaticMeshComponent|GetStaticMesh (Variables|Default|GetStaticMesh)))))))) (Math|Vector|MakeVector (Math|Conversions|ToFloat(Integer) (Variables|GridOptions|GetWidth)) (* (/ (Variables|GridOptions|GetHeight) 2) (Math|Float|Sqrt 3.0)) 1.0))) false false)
  (Rendering|Material|SetScalarParameterValueonMaterials (Variables|Default|GetStaticMesh) "WaveScalar" (Math|Conversions|ToFloat(Integer) (Variables|GridOptions|GetWidth))))

(fn UpdateInstancedStaticMesh
  (bind _water_tile_threshold (Variables|GridOptions|GetWater%20Tile%20Threshold))
  (bind _instancedstaticmesh (Variables|Default|GetInstancedStaticMesh))
  (bind _instance_index (Variables|Hidden|GetInstance%20Index))
  (bind _noisescale (Variables|Lvl1NoiseSettings|GetNoiseScale))
  (bind _noise_wrapper_lvl_1 (Variables|Hidden|GetNoise%20Wrapper%20Lvl%201))
  (bind _outinstancetransform (Components|InstancedStaticMesh|GetInstanceTransform _instancedstaticmesh _instance_index true))
  (bind _location (Math|Transform|BreakTransform _outinstancetransform))
  (bind (_x _y) (Class|KismetMathLibrary|BreakVector3f _location))
  (bind _returnvalue (* _x _noisescale))
  (bind _returnvalue_2 (* _y _noisescale))
  (bind _returnvalue_3 (Class|FastNoiseWrapper|GetNoise2D _noise_wrapper_lvl_1 _returnvalue _returnvalue_2))
  ;[0 1 0.015] Set Tile Height
  (if (<= _returnvalue_3 _water_tile_threshold)
    (Variables|Hidden|SetTile%20Height (- (* (Math|Float|Clamp(Float) _returnvalue_3 -1.0 _water_tile_threshold) (Variables|TileGenerationSettings|GetWater%20Tile%20Height%20Scalar)) (Variables|TileGenerationSettings|GetWater%20Tile%20Height%20Offset)))
    (else
      (Variables|Hidden|SetTile%20Height (Variables|GridOptions|GetLand%20Height))))
  (Components|InstancedStaticMesh|UpdateInstanceTransform (Variables|Default|GetInstancedStaticMesh) (Variables|Hidden|GetInstance%20Index) (Math|Transform|MakeTransform (+ (.Location (Math|Transform|BreakTransform (.OutInstanceTransform (Components|InstancedStaticMesh|GetInstanceTransform (Variables|Default|GetInstancedStaticMesh) (Variables|Hidden|GetInstance%20Index) true)))) (Math|Vector|MakeVector 0.0 0.0 (+ (* (Variables|Hidden|GetTile%20Height) (Variables|TileGenerationSettings|GetTile%20Height%20Strength)) (Variables|TileGenerationSettings|GetTile%20Height%20Offset))))) true false false)
  ;[0 1 0.9227] Add Tile Height to Custom Data
  (Components|InstancedStaticMesh|SetCustomDataValue (Variables|Default|GetInstancedStaticMesh) (Variables|Hidden|GetInstance%20Index) 0 (Variables|Hidden|GetTile%20Height) false))

(fn UpdateChildActors
  (params (Actor :type Child%20Actor%20Component%20Object%20Reference))
  (bind _noisescale (Variables|Lvl1NoiseSettings|GetNoiseScale))
  (LocalVariables|SetCurrent%20Actor Actor)
  ;[0 1 0.015] Set Tile Height
  (if (<= (Class|FastNoiseWrapper|GetNoise2D (Variables|Hidden|GetNoise%20Wrapper%20Lvl%201) (* (.X (Class|KismetMathLibrary|BreakVector3f (.Location (Math|Transform|BreakTransform (Transformation|GetWorldTransform (LocalVariables|GetCurrent%20Actor)))))) _noisescale) (* (.Y (Class|KismetMathLibrary|BreakVector3f (.Location (Math|Transform|BreakTransform (Transformation|GetWorldTransform (LocalVariables|GetCurrent%20Actor)))))) _noisescale)) 0.0)
    (Variables|Hidden|SetTile%20Height (- (* (Math|Float|Clamp(Float) (Class|FastNoiseWrapper|GetNoise2D (Variables|Hidden|GetNoise%20Wrapper%20Lvl%201) (* (.X (Class|KismetMathLibrary|BreakVector3f (.Location (Math|Transform|BreakTransform (Transformation|GetWorldTransform (LocalVariables|GetCurrent%20Actor)))))) _noisescale) (* (.Y (Class|KismetMathLibrary|BreakVector3f (.Location (Math|Transform|BreakTransform (Transformation|GetWorldTransform (LocalVariables|GetCurrent%20Actor)))))) _noisescale)) -1.0 0.0) 0.5) 0.8))
    (else
      (Variables|Hidden|SetTile%20Height (Variables|GridOptions|GetLand%20Height))))
  (Transformation|SetWorldLocation (LocalVariables|GetCurrent%20Actor) (+ (.Location (Math|Transform|BreakTransform (Transformation|GetWorldTransform (LocalVariables|GetCurrent%20Actor)))) (Math|Vector|MakeVector 0.0 0.0 (+ (* (Variables|Hidden|GetTile%20Height) (/ (Variables|TileGenerationSettings|GetTile%20Height%20Strength) 1e+02)) (Variables|TileGenerationSettings|GetTile%20Height%20Offset)))) false false)
  (return (LocalVariables|GetCurrent%20Actor)))

(fn SetNoiseWrappers
  ;[0 0.1983 1] Noise Wrapper
  (bind _returnvalue (Game|ConstructObjectfromClass "/Script/FastNoiseGenerator.FastNoiseWrapper"))
  (bind _output_get (Variables|Hidden|SetNoise%20Wrapper%20Lvl%201 _returnvalue))
  (Class|FastNoiseWrapper|SetupFastNoise _output_get (Variables|Lvl1NoiseSettings|GetNoise%20Type) (Variables|Lvl1NoiseSettings|GetSeed) (Variables|Lvl1NoiseSettings|GetFrequency) (Variables|Lvl1NoiseSettings|GetInterp) (Variables|Lvl1NoiseSettings|GetFractaltype) (Variables|Lvl1NoiseSettings|GetOctaves) (Variables|Lvl1NoiseSettings|GetLacunarity) (Variables|Lvl1NoiseSettings|GetGain) (Variables|Lvl1NoiseSettings|GetCellular%20Jitter) (Variables|Lvl1NoiseSettings|GetCellular%20Distance%20Function) (Variables|Lvl1NoiseSettings|GetCellular%20Return%20Type))
  ;[1 1 1] Noise Wrappers Decor
  (bind _keys (Utilities|Map|Keys (Variables|TileGenerationSettings|GetTile%20Tyes%20-%20Probabilities)))
  (for (_array_element _array_index) _keys
    (bind _returnvalue_2 (Game|ConstructObjectfromClass "/Script/FastNoiseGenerator.FastNoiseWrapper"))
    (Utilities|Map|Add (Variables|Default|GetNoise%20Wrappers%20Decor) _array_element _returnvalue_2)
    (Class|FastNoiseWrapper|SetupFastNoise _returnvalue_2 (Variables|DecorNoiseSettings|GetNoise%20Type%20Decor) (+ (Variables|DecorNoiseSettings|GetSeed%20Decor) _array_index) (Variables|DecorNoiseSettings|GetFrequency%20Decor) (Variables|DecorNoiseSettings|GetInterp%20Decor) (Variables|DecorNoiseSettings|GetFractal%20Type%20Decor) (Variables|DecorNoiseSettings|GetOctaves%20Decor) (Variables|DecorNoiseSettings|GetLacunarity%20Decor) (Variables|DecorNoiseSettings|GetGain%20Decor) (Variables|DecorNoiseSettings|GetCellular%20Jitter%20Decor) (Variables|DecorNoiseSettings|GetCellular%20Distance%20Function%20Decor) (Variables|DecorNoiseSettings|GetCellular%20Return%20Type%20Decor))))

(fn DebugTileTypesNumbers
  (bind _keys (Utilities|Map|Keys (Variables|TileGenerationSettings|GetTile%20Tyes%20-%20Probabilities)))
  (bind _output_get (LocalVariables|SetTile%20Type%20Count (Utilities|Map|MakeMap (.OutItem (Utilities|Array|Random _keys)) (+ 0 0))))
  (for _array_element _keys
    (Utilities|Map|Add _output_get _array_element 0))
  (bind _outactors (Actor|GetAllActorsOfClass (Variables|NormalTileOptions|GetHex%20Tile%20Class)))
  (for _array_element_2 _outactors
    (bind _asbp_hex_tile (Utilities|Casting|CastToBP_HexTile _array_element_2))
    (Utilities|Map|Add (LocalVariables|GetTile%20Type%20Count) (Variables|/Game/Blueprints/BP_HexTile.BP_HexTile_C|GetTile%20Type _asbp_hex_tile) (+ (.Value (Utilities|Map|Find (LocalVariables|GetTile%20Type%20Count) (Variables|/Game/Blueprints/BP_HexTile.BP_HexTile_C|GetTile%20Type _asbp_hex_tile))) 1)))
  (bind _keys_2 (Utilities|Map|Keys (LocalVariables|GetTile%20Type%20Count)))
  (for _array_element_3 _keys_2
    (Development|PrintString (Utilities|String|Append (Utilities|String|Append (Utilities|String|EnumtoString _array_element_3) " tile count =") (Utilities|String|ToString(Integer) (.Value (Utilities|Map|Find (LocalVariables|GetTile%20Type%20Count) _array_element_3)))) true true "(R=1.000000,G=0.000000,B=0.000000,A=1.000000)" 1e+01)))