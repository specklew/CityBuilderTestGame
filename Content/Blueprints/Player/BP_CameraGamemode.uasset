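; BP_CameraGamemode positions the player's camera pawn over the hex map when play begins.
; On BeginPlay it finds the BP_HexGenerator actor, stores it as Map, and stores player 0's pawn as CameraPawn.
; It then moves the pawn to the X and Y center of the map's actor bounds, at the InitialCameraHeight Z value.
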(event EventBeginPlay
  (bind _returnvalue (Actor|GetActorOfClass "/Game/Blueprints/Generator/BP_HexGenerator.BP_HexGenerator_C"))
  (Variables|Default|SetMap _returnvalue)
  (Variables|Default|SetCamera%20Pawn (Game|Player|GetPlayerPawn 0))
  (Transformation|SetActorLocationAndRotation (Variables|Default|GetCamera%20Pawn) (Math|Vector|MakeVector (.X (Class|KismetMathLibrary|BreakVector3f (.Origin (Collision|GetActorBounds (Variables|Default|GetMap) false false)))) (.Y (Class|KismetMathLibrary|BreakVector3f (.Origin (Collision|GetActorBounds (Variables|Default|GetMap) false false)))) (Variables|Default|GetInitial%20Camera%20Height))))

(fn ConstructionScript)