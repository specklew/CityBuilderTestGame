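; BP_PhysicsTree is a temporary tree actor that fades out and then removes itself.
; The construction script assigns the tree mesh and creates a dynamic material instance for each material slot.
; On BeginPlay, a timeline drives the "Fade Amount" scalar on every instance, then destroys the actor when it finishes.
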(event EventBeginPlay
  (bind _newtrack_0 (Timeline|Timeline Play)
    (:Update
      (for _array_element (Variables|Default|GetMaterial%20Instances)
        (Rendering|Material|SetScalarParameterValue _array_element "Fade Amount" _newtrack_0 :!class /Script/Engine.MaterialInstanceDynamic)))
    (:Finished
      (Actor|DestroyActor))))

(fn ConstructionScript
  (Components|StaticMesh|SetStaticMesh (Variables|Default|GetStaticMesh) (Variables|Default|GetTree%20Mesh))
  (for (_array_element _array_index) (Rendering|Material|GetMaterials (Variables|Default|GetStaticMesh))
    (bind _returnvalue (Rendering|Material|CreateDynamicMaterialInstance (Variables|Default|GetStaticMesh) _array_index _array_element "None" :!class /Script/Engine.PrimitiveComponent))
    (Utilities|Array|Add (Variables|Default|GetMaterial%20Instances) _returnvalue)))