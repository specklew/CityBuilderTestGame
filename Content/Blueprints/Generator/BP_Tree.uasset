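; BP_Tree is a damageable tree actor that picks a random look and turns into a physics tree when felled.
; The construction script adds a static mesh component with a random mesh from TreeMeshes and stores it as CurrentMesh.
; TakeDamage subtracts from TreeHP; at zero or below, it destroys the actor and spawns BP_PhysicsTree at the same transform with the same mesh.
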(fn ConstructionScript
  (bind _returnvalue (AddComponent|AddStaticMeshComponent false))
  (bind _output_get (Variables|Default|SetCurrent%20Mesh (.OutItem (Utilities|Array|Random (Variables|Default|GetTreeMeshes)))))
  (Components|StaticMesh|SetStaticMesh _returnvalue _output_get))

(fn TakeDamage
  (params (Damage :type Float%20%28double-precision%29))
  (Variables|Default|SetTreeHP (- (Variables|Default|GetTreeHP) Damage))
  (if (not (> (Variables|Default|GetTreeHP) 0.0))
    (Actor|DestroyActor)
    (Game|SpawnActorfromClass "/Game/Blueprints/Generator/BP_PhysicsTree.BP_PhysicsTree_C" (Transformation|GetActorTransform) "Undefined" "MultiplyWithRoot" 0 (Variables|Default|GetCurrent%20Mesh) 0)))