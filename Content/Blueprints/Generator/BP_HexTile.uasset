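; BP_HexTile is a procedural hex map tile that builds itself in its construction script using settings from its parent BP_HexGenerator.
; Noise sets the hexagon's height, with variable water depth and flat land, and feeds the material's Elevation parameter.
; Land type is the highest of per-type noises, each biased by an inverse error function of its probability.
; Forests add a ring of random trees, mountains one random mesh.
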(fn ConstructionScript
  (bind _asbp_hex_generator (Utilities|Casting|CastToBP_HexGenerator (Actor|GetParentActor self)))
  (bind _output_get (Variables|Default|SetGenerator _asbp_hex_generator))
  (Variables|Default|SetLocation (.Location (Math|Transform|BreakTransform (Transformation|GetActorTransform))))
  (CallFunction|SetTileHeight)
  (if (<= (Variables|Default|GetTile%20Height) (Variables|/Game/Blueprints/Generator/BP_HexGenerator.BP_HexGenerator_C|GetWater%20Tile%20Threshold _output_get))
    (CallFunction|SetMaterialParameters)
    (else
      (bind _keys (Utilities|Map|Keys (Variables|/Game/Blueprints/Generator/BP_HexGenerator.BP_HexGenerator_C|GetTile%20Tyes%20-%20Probabilities _output_get)))
      (for _array_element _keys
        (if (> (+ (Class|MathHelper|MyErfinvf (/ (.Value (Utilities|Map|Find (Variables|/Game/Blueprints/Generator/BP_HexGenerator.BP_HexGenerator_C|GetTile%20Tyes%20-%20Probabilities _output_get) _array_element)) 2.0)) (Class|FastNoiseWrapper|GetNoise2D (.Value (Utilities|Map|Find (Variables|/Game/Blueprints/Generator/BP_HexGenerator.BP_HexGenerator_C|GetNoise%20Wrappers%20Decor _output_get) _array_element)) (* (.X (Class|KismetMathLibrary|BreakVector3f (Variables|Default|GetLocation))) (Variables|/Game/Blueprints/Generator/BP_HexGenerator.BP_HexGenerator_C|GetNoise%20Scale%20Decor (Variables|Default|GetGenerator))) (* (.Y (Class|KismetMathLibrary|BreakVector3f (Variables|Default|GetLocation))) (Variables|/Game/Blueprints/Generator/BP_HexGenerator.BP_HexGenerator_C|GetNoise%20Scale%20Decor (Variables|Default|GetGenerator))))) (Variables|Default|GetTile%20Type%20Noise%20Value))
          (Variables|Default|SetTile%20Type%20Noise%20Value (+ (Class|MathHelper|MyErfinvf (/ (.Value (Utilities|Map|Find (Variables|/Game/Blueprints/Generator/BP_HexGenerator.BP_HexGenerator_C|GetTile%20Tyes%20-%20Probabilities _output_get) _array_element)) 2.0)) (Class|FastNoiseWrapper|GetNoise2D (.Value (Utilities|Map|Find (Variables|/Game/Blueprints/Generator/BP_HexGenerator.BP_HexGenerator_C|GetNoise%20Wrappers%20Decor _output_get) _array_element)) (* (.X (Class|KismetMathLibrary|BreakVector3f (Variables|Default|GetLocation))) (Variables|/Game/Blueprints/Generator/BP_HexGenerator.BP_HexGenerator_C|GetNoise%20Scale%20Decor (Variables|Default|GetGenerator))) (* (.Y (Class|KismetMathLibrary|BreakVector3f (Variables|Default|GetLocation))) (Variables|/Game/Blueprints/Generator/BP_HexGenerator.BP_HexGenerator_C|GetNoise%20Scale%20Decor (Variables|Default|GetGenerator))))))
          (Variables|Default|SetTile%20Type _array_element)))
      (switch Utilities|FlowControl|Switch|SwitchonTileType (Variables|Default|GetTile%20Type)
        (:NewEnumerator0
          (CallFunction|InstantiateForest))
        (:NewEnumerator1
          (CallFunction|InstantiateMountain))
        (:NewEnumerator2
          _))
      (CallFunction|SetMaterialParameters))))

(fn SetTileHeight
  (bind _returnvalue (Transformation|GetActorTransform))
  (bind _generator (Variables|Default|GetGenerator))
  (bind _generator_2 (Variables|Default|GetGenerator))
  (bind _generator_3 (Variables|Default|GetGenerator))
  (bind _location (Math|Transform|BreakTransform _returnvalue))
  (bind _noise_wrapper_lvl_1 (Variables|/Game/Blueprints/Generator/BP_HexGenerator.BP_HexGenerator_C|GetNoise%20Wrapper%20Lvl%201 _generator))
  (bind _noisescale (Variables|/Game/Blueprints/Generator/BP_HexGenerator.BP_HexGenerator_C|GetNoiseScale _generator_2))
  (bind (_x _y) (Class|KismetMathLibrary|BreakVector3f _location))
  (bind _returnvalue_2 (* _x _noisescale))
  (bind _returnvalue_3 (* _y _noisescale))
  (bind _returnvalue_4 (Class|FastNoiseWrapper|GetNoise2D _noise_wrapper_lvl_1 _returnvalue_2 _returnvalue_3))
  ;[0 1 0.015] Set Tile Height
  (if (<= _returnvalue_4 (Variables|/Game/Blueprints/Generator/BP_HexGenerator.BP_HexGenerator_C|GetWater%20Tile%20Threshold (Variables|Default|GetGenerator)))
    (Variables|Default|SetTile%20Height (- (* (Math|Float|Clamp(Float) _returnvalue_4 -1.0) (Variables|/Game/Blueprints/Generator/BP_HexGenerator.BP_HexGenerator_C|GetWater%20Tile%20Height%20Scalar _generator_3)) (Variables|/Game/Blueprints/Generator/BP_HexGenerator.BP_HexGenerator_C|GetWater%20Tile%20Height%20Offset _generator_3)))
    (else
      (Variables|Default|SetTile%20Height (Variables|/Game/Blueprints/Generator/BP_HexGenerator.BP_HexGenerator_C|GetLand%20Height _generator_3))))
  (Transformation|SetWorldTransform (Variables|Default|GetHexagon) (Math|Transform|MakeTransform (+ (.Location (Math|Transform|BreakTransform (Transformation|GetActorTransform))) (Math|Vector|MakeVector 0.0 0.0 (+ (* (Variables|Default|GetTile%20Height) (Variables|/Game/Blueprints/Generator/BP_HexGenerator.BP_HexGenerator_C|GetTile%20Height%20Strength _generator_3)) (Variables|/Game/Blueprints/Generator/BP_HexGenerator.BP_HexGenerator_C|GetTile%20Height%20Offset _generator_3))))) false false))

(fn SetMaterialParameters
  (Rendering|Material|SetScalarParameterValueonMaterials (Variables|Default|GetHexagon) "Elevation" (Variables|Default|GetTile%20Height)))

(fn InstantiateMountain
  (bind _returnvalue (AddComponent|AddStaticMeshComponent false (Math|Transform|MakeTransform (.Location (Math|Transform|BreakTransform (Transformation|GetRelativeTransform (Variables|Default|GetHexagon)))) "0, 0, 0" (Math|Conversions|ToVector(Float) (Variables|Default|GetMountains%20Scale)))))
  (Components|StaticMesh|SetStaticMesh _returnvalue (.OutItem (Utilities|Array|Random (Variables|Default|GetMountainMeshes)))))

(fn InstantiateForest
  (bind _generator (Variables|Default|GetGenerator))
  (for _index (range 0 (- (Variables|/Game/Blueprints/Generator/BP_HexGenerator.BP_HexGenerator_C|GetTrees%20In%20Forest _generator) 1))
    (LocalVariables|SetX%20Tree%20Offset (* (Math|Trig|Sin(Degrees) (+ (LocalVariables|GetCurrent%20Angle) (Variables|/Game/Blueprints/Generator/BP_HexGenerator.BP_HexGenerator_C|GetTree%20Spawn%20Angle%20Offset _generator))) (Variables|/Game/Blueprints/Generator/BP_HexGenerator.BP_HexGenerator_C|GetTree%20Spawn%20Offset _generator)))
    (LocalVariables|SetY%20Tree%20Offset (* (Math|Trig|Cos(Degrees) (+ (LocalVariables|GetCurrent%20Angle) (Variables|/Game/Blueprints/Generator/BP_HexGenerator.BP_HexGenerator_C|GetTree%20Spawn%20Angle%20Offset _generator))) (Variables|/Game/Blueprints/Generator/BP_HexGenerator.BP_HexGenerator_C|GetTree%20Spawn%20Offset _generator)))
    (bind _returnvalue (AddComponent|AddStaticMeshComponent false (Math|Transform|MakeTransform (+ (Math|Vector|MakeVector (LocalVariables|GetX%20Tree%20Offset) (LocalVariables|GetY%20Tree%20Offset) 0.0) (.Location (Math|Transform|BreakTransform (Transformation|GetRelativeTransform (Variables|Default|GetHexagon))))) "0, 0, 0" (Math|Conversions|ToVector(Float) (Variables|Default|GetTrees%20Scale)))))
    (Components|StaticMesh|SetStaticMesh _returnvalue (.OutItem (Utilities|Array|Random (Variables|Default|GetTreeMeshes))))
    (LocalVariables|SetCurrent%20Angle (+ (LocalVariables|GetCurrent%20Angle) (/ (LocalVariables|GetFull%20360) (Variables|/Game/Blueprints/Generator/BP_HexGenerator.BP_HexGenerator_C|GetTrees%20In%20Forest (Variables|Default|GetGenerator)))))))